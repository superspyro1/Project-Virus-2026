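; Enemy character that chases the player, deals damage in range and announces its death through CallEnemyDied when destroyed.
; Tick drives simple AI movement toward the player pawn, while capsule overlaps toggle collision modes and start a re-arming attack timer.
; Incoming damage is reduced by Defense, then fed to ACHealth and a health bar widget.
; Difficulty tiers set combat, health and regen stats, with Difficulty also multiplying speed and outgoing damage.
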(event OnComponentBeginOverlap(CapsuleComponent)
  (params (OverlappedComponent :type Primitive%20Component%20Object%20Reference) (OtherActor :type Actor%20Object%20Reference) (OtherComp :type Primitive%20Component%20Object%20Reference) (OtherBodyIndex :type Integer) (bFromSweep :type Boolean) (SweepResult :type Hit%20Result%20Structure%20%28by%20ref%29))
  (if (Actor|ActorHasTag OtherActor "Player")
    (Collision|SetCollisionEnabled (Variables|Default|GetCube) "QueryAndPhysics")
    (Variables|Default|SetTargetActor OtherActor)
    (Variables|Default|SetbInRange true)
    (CallFunction|StartAttackTimer)
    (elif (Actor|ActorHasTag OtherActor "Enemy")
      (Collision|SetCollisionEnabled (Variables|Default|GetCube) "QueryOnly"))))

(event OnComponentEndOverlap(CapsuleComponent)
  (params (OverlappedComponent :type Primitive%20Component%20Object%20Reference) (OtherActor :type Actor%20Object%20Reference) (OtherComp :type Primitive%20Component%20Object%20Reference) (OtherBodyIndex :type Integer))
  (if (Actor|ActorHasTag OtherActor "Player")
    (Variables|Default|SetTargetActor 0)
    (Variables|Default|SetbInRange false)))

(event Custom|StartAttackTimer
  (CallFunction|UpdateDamage)
  (bind _currentattacktime (CallFunction|UpdateAttackTime))
  (bind _returnvalue (Utilities|Time|SetTimerbyEvent (delegate Custom|AttackTarget) _currentattacktime))
  (Variables|Default|SetAttackingHandle _returnvalue))

(event Custom|AttackTarget
  (if (Variables|Default|GetbInRange)
    (Class|BPICombat|DealDamage(Message) (Variables|Default|GetTargetActor) (Variables|Default|GetFinalDamage) self)
    (CallFunction|StartAttackTimer)
    (else
      (Utilities|Time|ClearandInvalidateTimerbyHandle (Variables|Default|GetAttackingHandle)))))

(event EventBeginPlay
  (bind _aswbp_health (Utilities|Casting|CastToWBP_Health (UserInterface|GetUserWidgetObject (Variables|Default|GetHealthBar))))
  (bind _output_get (Variables|Default|SetHealthWidget _aswbp_health))
  (Widget|SetVisibility _output_get "Hidden")
  (Utilities|FlowControl|Delay 0.1)
  (Collision|SetActorEnableCollision true))

(event EventDealDamage
  (params (Amount :type Float%20%28double-precision%29) (Source :type Actor%20Object%20Reference))
  (bind _ac_health (Variables|Default|GetAC_Health))
  (bind _healthwidget (Variables|Default|GetHealthWidget))
  (bind _finaldamage (CallFunction|CalculateDamage Amount))
  (bind _dead_ (Default|RemoveHealth _ac_health _finaldamage))
  (if _dead_
    (Actor|DestroyActor)
    (else
      (if (Default|CheckHealth _ac_health)
        (Widget|SetVisibility _healthwidget "Visible")
        (else
          (Widget|SetVisibility _healthwidget "Hidden")))
      (CallFunction|UpdateHealthWidget))))

(event EventDestroyed
  (Default|CallEnemyDied))

(event EventTick
  (params (DeltaSeconds :type Float%20%28single-precision%29))
  (Utilities|FlowControl|Delay 0.1)
  (AI|Navigation|SimpleMovetoLocation (AI|GetAIController self) (Transformation|GetActorLocation (Game|Player|GetPlayerPawn 0))))

(fn ConstructionScript)

(fn CalculateDamage
  (params (IncomingDamage :type Float%20%28double-precision%29))
  (return (Math|Float|Clamp(Float) (- IncomingDamage (Variables|Default|GetDefense)) 0.0 1e+12)))

(fn UpdateHealthWidget
  (Default|UpdateHealthBar (Variables|Default|GetHealthWidget) (Default|CalculateHealth (Variables|Default|GetAC_Health))))

(fn DamageIndicator
  (Niagara|SpawnSystematLocation "/Game/Blueprints/FX/Niagara/NS_HitDetection.NS_HitDetection" (Transformation|GetActorLocation) (Math|Random|RandomRotator false)))

(fn UpdateStartingStats
  (params (Difficulty :type Float%20%28double-precision%29))
  (if (>= Difficulty 2.0)
    (if (>= Difficulty 4.0)
      (if (>= Difficulty 6.0)
        (if (>= Difficulty 8.0)
          (if (>= Difficulty 1e+01)
            (CallFunction|AssignStats Difficulty 7e+02 1e+01 0.8 1.4 4e+01 3.2e+03 3e+01)
            (else
              (CallFunction|AssignStats Difficulty 6e+02 5.0 0.8 1.4 2e+01 1.6e+03 2e+01)))
          (else
            (CallFunction|AssignStats Difficulty 5e+02 5.0 0.9 1.2 15.0 8e+02 1e+01)))
        (else
          (CallFunction|AssignStats Difficulty 4e+02 5.0 0.9 1.2 1e+01 4e+02 5.0)))
      (else
        (CallFunction|AssignStats Difficulty 4e+02 5.0 1.0 1.0 5.0 2e+02 2.0)))
    (else
      (CallFunction|AssignStats Difficulty 4e+02 5.0 1.0 1.0 0.0 1e+02 1.0))))

(fn AssignStats
  (params (Difficulty :type Float%20%28double-precision%29) (Speed :type Float%20%28double-precision%29) (Damage :type Float%20%28double-precision%29) (Cooldown :type Float%20%28double-precision%29) (Duration :type Float%20%28double-precision%29) (Defense :type Float%20%28double-precision%29) (MaxHealth :type Float%20%28double-precision%29) (RegenRate :type Float%20%28double-precision%29))
  (bind _ac_health (Variables|Default|GetAC_Health))
  (bind _output_get (Variables|Default|SetDifficulty Difficulty))
  (CallFunction|CalculateNewSpeed _output_get Speed)
  (Variables|Default|SetDamage Damage)
  (Variables|Default|SetCooldown Cooldown)
  (Variables|Default|SetDuration Duration)
  (Variables|Default|SetDefense Defense)
  (Default|SetMaxHealth _ac_health MaxHealth)
  (Default|UpdateRegenRate _ac_health RegenRate))

(fn CalculateNewSpeed
  (params (Difficulty :type Float%20%28double-precision%29) (NewSpeed :type Float%20%28double-precision%29))
  (Variables|/Script/Engine.CharacterMovementComponent|SetMaxWalkSpeed (Variables|Character|GetCharacterMovement) (* NewSpeed Difficulty)))

(fn UpdateDamage
  (Variables|Default|SetFinalDamage (* (Variables|Default|GetDamage) (Variables|Default|GetDifficulty)))
  (return))

(fn UpdateAttackTime
  (bind _output_get (Variables|Default|SetFinalAttackTime (* (Variables|Default|GetAttackTime) (Variables|Default|GetCooldown))))
  (return _output_get))