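; Wave spawner that runs the enemy wave loop, starting a wave each time the player selects an upgrade.
; Each wave's groups come from WaveMap and spawn sequentially on a timer at random BP_Enemy_Spawn actors, scaled by a difficulty multiplier.
; Enemy death events decrement a live count that triggers the player's level-up at zero.
; When WaveMap has no entry for the next wave, the player achieves victory.
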(event Custom|RefPlayer
  ;[0.15 0.15 0.15 0.5] Hard References
  (bind _asbpc_player_character (Utilities|Casting|CastToBPC_PlayerCharacter (Game|Player|GetPlayerPawn 0))
    (:then
      (bind _output_get (Variables|Default|SetPlayerRef _asbpc_player_character))
      (EventDispatchers|BindEventtoOnUpgradeSelected _output_get (delegate Custom|NewWave)))
    (:CastFailed
      (Utilities|FlowControl|DelayUntilNextTick)
      (CallFunction|RefPlayer))))

(event Custom|RefSpawners
  ;[0.15 0.15 0.15 0.5] Hard References
  (bind _outactors (Actor|GetAllActorsOfClass "/Game/Blueprints/Spawners/BP_Enemy_Spawn.BP_Enemy_Spawn_C"))
  (Variables|Default|SetSpawners _outactors))

(event Custom|NewWave
  (params (CardType :type E_CardType%20Enum :default "NewEnumerator0") (AbilityData :type S%20Ability%20Structure) (UpgradeData :type S%20Stat%20Upgrade%20Structure))
  ;[0.15 0.15 0.15 0.5] New Wave
  (CallFunction|RefSpawners)
  (bind _result (Math|Integer|IncrementInt (Variables|Default|GetCurrentWave))
    (:%20%20
      (if (.ReturnValue (Utilities|Map|Find (Variables|Default|GetWaveMap) _result))
        (Variables|Default|SetEnemies (Utilities|Struct|BreakS_WaveEnemies (.Value (Utilities|Map|Find (Variables|Default|GetWaveMap) _result))))
        (CallFunction|CheckWaveGroup)
        (else
          (Default|AchieveVictory (Variables|Default|GetPlayerRef)))))))

(event Custom|StartWaveCounter
  ;[0.15 0.15 0.15 0.5] Spawn Wave
  (bind _returnvalue (Utilities|Time|SetTimerbyEvent (delegate Custom|SpawnWave) (Variables|Default|GetSpawn%20Delay)))
  (Variables|Default|SetWaveTimerHandle _returnvalue))

(event Custom|SpawnWave
  ;[0.15 0.15 0.15 0.5] Spawn Wave
  (Utilities|Time|ClearandInvalidateTimerbyHandle (Variables|Default|GetWaveTimerHandle))
  (CallFunction|SpawnEnemy))

(event Custom|CheckEnemiesRemaining
  (bind _result (Math|Integer|DecrementInt (Variables|Default|GetRemainingEnemies))
    (:%20%20
      (if (<= _result 0)
        (Default|LevelUp (Variables|Default|GetPlayerRef))))))

(event Custom|SpawnEnemy
  (if (> (Variables|Default|GetSpawnsRemaining) 0)
    (Math|Integer|DecrementInt (Variables|Default|GetSpawnsRemaining)
      (:%20%20
        (bind _returnvalue (Game|SpawnActorfromClass (Variables|Default|GetEnemy%20Class) (CallFunction|CalculateSpawnLoc) "AlwaysSpawn" "MultiplyWithRoot" 0 0))
        (Utilities|IsValid _returnvalue
          (:Is%20Valid
            (Default|UpdateStartingStats _returnvalue (Variables|Default|GetDifficulty%20Multiplier))
            (EventDispatchers|BindEventtoEnemyDied _returnvalue (delegate Custom|CheckEnemiesRemaining))
            (Math|Integer|IncrementInt (Variables|Default|GetRemainingEnemies)
              (:%20%20
                _)))
          (:Is%20Not%20Valid
            (Math|Integer|IncrementInt (Variables|Default|GetSpawnsRemaining)
              (:%20%20
                _))))
        (CallFunction|StartWaveCounter)))
    (else
      (CallFunction|CheckWaveGroup))))

(event Custom|CheckWaveGroup
  (bind _enemies (Variables|Default|GetEnemies))
  (bind _output (Utilities|Array|Get(acopy) _enemies))
  (bind (_enemyclass _quantity _spawndelay _difficultymultiplier) (Utilities|Struct|BreakS_WaveGroup _output))
  (bind _groupremaining (CallFunction|CheckWaveLength))
  (if _groupremaining
    (Utilities|FlowControl|DelayUntilNextTick)
    (Variables|Default|SetEnemy%20Class _enemyclass)
    (Variables|Default|SetSpawnsRemaining _quantity)
    (Variables|Default|SetSpawn%20Delay _spawndelay)
    (Variables|Default|SetDifficulty%20Multiplier _difficultymultiplier)
    (Utilities|FlowControl|DelayUntilNextTick)
    (Utilities|Array|RemoveIndex (Variables|Default|GetEnemies))
    (CallFunction|StartWaveCounter)))

(event EventBeginPlay
  (CallFunction|RefPlayer))

(fn ConstructionScript)

(fn CalculateSpawnLoc
  (bind _spawners (Variables|Default|GetSpawners))
  (bind _outitem (Utilities|Array|Random _spawners))
  (bind _returnvalue (Transformation|GetActorTransform _outitem))
  (return (Math|Transform|MakeTransform (Math|Vector|MakeVector (.x (.location _returnvalue)) (.y (.location _returnvalue)) (+ (.z (.location _returnvalue)) 1.0)) (.rotation _returnvalue) (.scale _returnvalue))))

(fn CheckWaveLength
  (if (> (Utilities|Array|Length (Variables|Default|GetEnemies)) 0)
    (return true)
    (else
      (return false))))