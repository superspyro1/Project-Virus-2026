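; Antibody Burst ability that keeps four antibody projectiles orbiting on a spline path, with damage derived from the player's stats.
; A looping timeline moves four evenly spaced orbit points along the spline, and a projectile is spawned attached to each.
; Each spawn recalculates damage from base antibody damage and player damage and multiplier.
; Orbit points passed to SpawnNewAntibody queue for respawn, refilled one per cooldown by a looping timer.
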(event Custom|SpawnAntibody
  (params (OrbitLocation :type Scene%20Component%20Object%20Reference))
  (CallFunction|CalculateDamage)
  (Utilities|IsValid OrbitLocation
    (:Is%20Valid
      (bind _returnvalue (Game|SpawnActorfromClass "/Game/Blueprints/Components/Abilities/AntibodyBurst/BP_AntibodyProjectile.BP_AntibodyProjectile_C" (Transformation|GetRelativeTransform OrbitLocation) "AlwaysSpawn" "MultiplyWithRoot" 0 0))
      (Utilities|IsValid _returnvalue
        (:Is%20Valid
          (Default|AssignValues _returnvalue (Variables|Default|GetFinalDamage) (Variables|Default|GetCooldown) self OrbitLocation)
          (Transformation|AttachComponentToComponent _returnvalue OrbitLocation "None" "SnapToTarget" "KeepWorld" "KeepWorld" true))))))

(event Custom|StartSpline
  (bind _newtrack_0 (Timeline|Timeline PlayFromStart)
    (:Update
      (for (_array_element _array_index) (Variables|Default|GetOrbitLocs)
        (Transformation|SetRelativeLocationAndRotation _array_element (+ (Spline|GetLocationatDistanceAlongSpline (Variables|Default|GetAntibodyBurstOrbitPath) (* (Math|Float|%(Float) (+ (* _array_index 0.25) _newtrack_0) 1.0) (Spline|GetSplineLength (Variables|Default|GetAntibodyBurstOrbitPath))) "Local") "0.000000,-200.000000,0.000000") (Spline|GetRotationatDistanceAlongSpline (Variables|Default|GetAntibodyBurstOrbitPath) (* (Math|Float|%(Float) (+ (* _array_index 0.25) _newtrack_0) 1.0) (Spline|GetSplineLength (Variables|Default|GetAntibodyBurstOrbitPath))) "Local") false false))
      (CallFunction|SpawnInitialAntibodies))
    (:Finished
      (CallFunction|StartSpline))))

(event Custom|SpawnNewAntibody
  (params (OrbitLoc :type Scene%20Component%20Object%20Reference))
  (Utilities|Array|Add (Variables|Default|GetRespawnLocs) OrbitLoc)
  (if (not (Utilities|Time|IsValidTimerHandle (Variables|Default|GetRespawnTimerHandle)))
    (bind _returnvalue (Utilities|Time|SetTimerbyEvent (delegate Custom|RespawnProjectile) (Variables|Default|GetCooldown) true))
    (Variables|Default|SetRespawnTimerHandle _returnvalue)))

(event Custom|SetOrbitLocs
  (Variables|Default|SetOrbitLocs (Utilities|Array|MakeArray (Variables|Default|GetOrbitLoc1) (Variables|Default|GetOrbitLoc2) (Variables|Default|GetOrbitLoc3) (Variables|Default|GetOrbitLoc4)))
  (Utilities|FlowControl|DelayUntilNextTick)
  (CallFunction|CalculateDamage)
  (Utilities|FlowControl|DelayUntilNextTick)
  (CallFunction|StartSpline))

(event Custom|SpawnInitialAntibodies
  (Utilities|FlowControl|DoOnce false
    (:Completed
      (for _array_element (Variables|Default|GetOrbitLocs)
        (CallFunction|SpawnAntibody _array_element)))))

(event Custom|RespawnProjectile
  (if (> (Utilities|Array|Length (Variables|Default|GetRespawnLocs)) -1)
    (CallFunction|SpawnAntibody (Utilities|Array|Get(acopy) (Variables|Default|GetRespawnLocs)))
    (Utilities|Array|RemoveIndex (Variables|Default|GetRespawnLocs))
    (else
      (Utilities|Time|ClearandInvalidateTimerbyHandle (Variables|Default|GetRespawnTimerHandle)))))

(event Custom|RefPlayer
  (bind _asbpc_player_character (Utilities|Casting|CastToBPC_PlayerCharacter (Game|Player|GetPlayerPawn 0))
    (:then
      (Variables|Default|SetPlayerRef _asbpc_player_character))
    (:CastFailed
      (Utilities|FlowControl|DelayUntilNextTick)
      (CallFunction|RefPlayer))))

(event EventBeginPlay
  (CallFunction|SetOrbitLocs)
  (CallFunction|RefPlayer))

(fn ConstructionScript)

(fn GetStats
  (params (Damage :type Float%20%28double-precision%29) (DamageMultiplier :type Float%20%28double-precision%29) (Cooldown :type Float%20%28double-precision%29) (Duration :type Float%20%28double-precision%29))
  (Variables|Default|SetDamage Damage)
  (Variables|Default|SetDamage%20Multiplier DamageMultiplier)
  (Variables|Default|SetCooldown Cooldown)
  (Variables|Default|SetDuration Duration))

(fn CalculateDamage
  (bind (_newmultiplier _newdamage) (CallFunction|UpdateStats))
  (bind _output_get (Variables|Default|SetFinalDamage (* _newmultiplier (+ _newdamage (Variables|Default|GetAntibodyDamage)))))
  (return _output_get))

(fn UpdateStats
  (bind _playerref (Variables|Default|GetPlayerRef))
  (bind (_damage _damagemultiplier) (Default|GetDamage _playerref))
  (bind _output_get (Variables|Default|SetDamage _damage))
  (bind _output_get_2 (Variables|Default|SetDamage%20Multiplier _damagemultiplier))
  (return _output_get_2 _output_get))