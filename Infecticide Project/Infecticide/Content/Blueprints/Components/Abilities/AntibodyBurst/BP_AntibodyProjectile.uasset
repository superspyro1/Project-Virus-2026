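; Projectile for the Antibody Burst ability that waits attached to its host, then launches at enemies and damages them on contact.
; AssignValues sets damage, host and orbit slot, then enables collision and detection after a cooldown.
; An enemy entering EnemyDetection detaches it and sets its velocity toward that enemy's current position, without homing.
; HitDetection deals damage and destroys it; destruction tells the host to spawn a replacement in the same slot.
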(event OnComponentBeginOverlap(EnemyDetection)
  (params (OverlappedComponent :type Primitive%20Component%20Object%20Reference) (OtherActor :type Actor%20Object%20Reference) (OtherComp :type Primitive%20Component%20Object%20Reference) (OtherBodyIndex :type Integer) (bFromSweep :type Boolean) (SweepResult :type Hit%20Result%20Structure%20%28by%20ref%29))
  (if (Variables|Default|GetbOrbiting)
    (Utilities|IsValid OtherActor
      (:Is%20Valid
        (if (Actor|ActorHasTag OtherActor "Enemy")
          (CallFunction|DetachfromHost)
          (bind _output_get (Variables|Default|SetTargetEnemy OtherActor))
          (Variables|/Script/Engine.MovementComponent|SetVelocity (Variables|Default|GetProjectileMovement) (* (Math|Vector|GetUnitDirection(Vector) (Transformation|GetActorLocation self) (Transformation|GetActorLocation _output_get)) (Variables|Default|GetProjectileSpeed))))))))

(event OnComponentBeginOverlap(HitDetection)
  (params (OverlappedComponent :type Primitive%20Component%20Object%20Reference) (OtherActor :type Actor%20Object%20Reference) (OtherComp :type Primitive%20Component%20Object%20Reference) (OtherBodyIndex :type Integer) (bFromSweep :type Boolean) (SweepResult :type Hit%20Result%20Structure%20%28by%20ref%29))
  (Utilities|IsValid OtherActor
    (:Is%20Valid
      (if (Actor|ActorHasTag OtherActor "Enemy")
        (Class|BPICombat|DealDamage(Message) OtherActor (Variables|Default|GetDamage) self)
        (Utilities|FlowControl|DelayUntilNextTick)
        (Actor|DestroyActor)))))

(event Custom|RefPlayer
  (bind _asbpc_player_character (Utilities|Casting|CastToBPC_PlayerCharacter (Game|Player|GetPlayerPawn 0)))
  (Variables|Default|SetPlayerRef _asbpc_player_character))

(event Custom|StartOrbiting
  (params (Cooldown :type Float%20%28double-precision%29))
  (Utilities|FlowControl|Delay Cooldown)
  (Variables|Default|SetbOrbiting true)
  (Collision|SetActorEnableCollision true))

(event EventBeginPlay
  (CallFunction|RefPlayer))

(event EventDestroyed
  (CallFunction|TriggerSpawn))

(fn ConstructionScript)

(fn DetachfromHost
  (Transformation|DetachFromActor "KeepWorld" "KeepWorld" "KeepWorld"))

(fn TriggerSpawn
  (Default|SpawnNewAntibody (Variables|Default|GetHost) (Variables|Default|GetOrbitLoc)))

(fn AssignValues
  (params (NewDamage :type Float%20%28double-precision%29) (Cooldown :type Float%20%28double-precision%29) (Host :type BP%20Antibody%20Burst%20Object%20Reference) (OrbitLoc :type Scene%20Component%20Object%20Reference))
  (Variables|Default|SetDamage NewDamage)
  (bind _output_get (Variables|Default|SetCooldown Cooldown))
  (Variables|Default|SetHost Host)
  (Variables|Default|SetOrbitLoc OrbitLoc)
  (CallFunction|StartOrbiting _output_get)
  (return))