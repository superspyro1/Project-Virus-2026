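; Ability component that gives the player character an Antibody Burst by spawning a BP_AntibodyBurst actor on it.
; On BeginPlay it looks up the player character, retrying each tick until the cast succeeds, then caches the reference.
; It passes the player's damage and timing stats to the spawned burst and attaches it to the player, snapped to location.
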(event Custom|RefPlayer
  (bind _asbpc_player_character (Utilities|Casting|CastToBPC_PlayerCharacter (Game|GetPlayerCharacter 0))
    (:then
      (bind _output_get (Variables|Default|SetPlayerRef _asbpc_player_character))
      (CallFunction|SpawnAntibodyReaction _output_get))
    (:CastFailed
      (Utilities|FlowControl|DelayUntilNextTick)
      (CallFunction|RefPlayer))))

(event Custom|SpawnAntibodyReaction
  (params (ActorRef :type Actor%20Object%20Reference))
  (bind _playerref (Variables|Default|GetPlayerRef))
  (bind (_damage _damagemultiplier) (Default|GetDamage _playerref))
  (bind (_cooldown _duration) (Default|GetTiming _playerref))
  (bind _returnvalue (Game|SpawnActorfromClass "/Game/Blueprints/Components/Abilities/AntibodyBurst/BP_AntibodyBurst.BP_AntibodyBurst_C" (Transformation|GetActorTransform ActorRef) "AlwaysSpawn" "MultiplyWithRoot" 0 0))
  (Default|GetStats _returnvalue _damage _damagemultiplier _cooldown _duration)
  (Transformation|AttachActorToActor _returnvalue ActorRef "None" "SnapToTarget" "KeepRelative" "KeepWorld" true))

(event EventBeginPlay
  (CallFunction|RefPlayer))