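; Spike body ability component that periodically makes the player negate damage while a Niagara spike effect plays on their mesh.
; On BeginPlay it casts the owner to BPC_PlayerCharacter, attaches the effect and starts activation.
; Two timers alternate active and cooldown phases, toggling NegateDamage and the effect.
; Each phase change recalculates damage, duration and cooldown from player stats, though the computed damage is not applied here.
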(event Custom|TurnOnSpikes
  (Utilities|Time|ClearandInvalidateTimerbyHandle (Variables|Default|GetCooldownTimerHandle))
  (CallFunction|ActivateSpikes))

(event Custom|BeginCooldown
  (CallFunction|UpdateStats)
  (bind _output_get (Variables|/Game/Blueprints/BPC_PlayerCharacter.BPC_PlayerCharacter_C|SetbNegateDamage (Variables|Default|GetPlayerRef) false))
  (Variables|Default|SetbActivated _output_get)
  (bind _returnvalue (Utilities|Time|SetTimerbyEvent (delegate Custom|TurnOnSpikes) (Variables|Time|GetCooldown)))
  (Variables|Default|SetCooldownTimerHandle _returnvalue)
  (Components|Activation|Deactivate (Variables|Default|GetActivationEffect)))

(event Custom|ActivateSpikes
  (CallFunction|UpdateStats)
  (bind _output_get (Variables|/Game/Blueprints/BPC_PlayerCharacter.BPC_PlayerCharacter_C|SetbNegateDamage (Variables|Default|GetPlayerRef) true))
  (Variables|Default|SetbActivated _output_get)
  (bind _returnvalue (Utilities|Time|SetTimerbyEvent (delegate Custom|TurnOffSpikes) (Variables|Time|GetDuration)))
  (Variables|Default|SetActivatedTimerHandle _returnvalue)
  (Components|Activation|Activate (Variables|Default|GetActivationEffect) true))

(event Custom|TurnOffSpikes
  (Utilities|Time|ClearandInvalidateTimerbyHandle (Variables|Default|GetActivatedTimerHandle))
  (CallFunction|BeginCooldown))

(event Custom|RefPlayer
  (bind _asbpc_player_character (Utilities|Casting|CastToBPC_PlayerCharacter (Components|GetOwner)))
  (bind _output_get (Variables|Default|SetPlayerRef _asbpc_player_character))
  (bind _returnvalue (Niagara|SpawnSystemAttached "/Game/Blueprints/FX/Niagara/NS_SpikeBody.NS_SpikeBody" (Variables|/Script/Engine.Character|GetMesh _output_get) "None" "0, 0, 0" "0, 0, 0" "SnapToTarget" false false))
  (Variables|Default|SetActivationEffect _returnvalue)
  (CallFunction|ActivateSpikes))

(event Custom|UpdateStats
  (bind _playerref (Variables|Default|GetPlayerRef))
  (Damage|CalculateDamage (Variables|/Game/Blueprints/BPC_PlayerCharacter.BPC_PlayerCharacter_C|GetDamageMultiplier _playerref) (Variables|/Game/Blueprints/BPC_PlayerCharacter.BPC_PlayerCharacter_C|GetDamage _playerref))
  (Time|CalculateTime (Variables|/Game/Blueprints/BPC_PlayerCharacter.BPC_PlayerCharacter_C|GetCooldown _playerref) (Variables|/Game/Blueprints/BPC_PlayerCharacter.BPC_PlayerCharacter_C|GetDuration _playerref)))

(event EventBeginPlay
  (CallFunction|RefPlayer))

(fn CalculateDamage
  (params (Multiplier :type Float%20%28double-precision%29) (Damage :type Float%20%28double-precision%29))
  (Variables|Damage|SetFinalDamage (* Multiplier (+ Damage (Variables|Damage|GetSpikeDamage))))
  (return))

(fn CalculateTime
  (params (CooldownMultiplier :type Float%20%28double-precision%29) (DurationMultiplier :type Float%20%28double-precision%29))
  (Variables|Time|SetCooldown (* CooldownMultiplier (Variables|Time|GetBaseCooldown)))
  (Variables|Time|SetDuration (* DurationMultiplier (Variables|Time|GetBaseDuration)))
  (return))