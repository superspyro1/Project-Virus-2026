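; Health component for Player- and Enemy-tagged actors, caching a typed owner reference on BeginPlay.
; It stores clamped current health, exposes percent and below-max checks, and reports when removal reaches zero.
; Nonzero regen-rate updates start a looping one-second timer that calls the player's HealDamage; the enemy branch is empty.
; Negative rates flag Injured but still regenerate, while updating to zero returns without clearing the timer.
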(event Custom|RegenHealth
  (bind _playerref (Variables|Default|GetPlayerRef))
  (Utilities|IsValid _playerref
    (:Is%20Valid
      (Default|HealDamage _playerref (Variables|Regen|GetRegenRate)))
    (:Is%20Not%20Valid
      (Utilities|IsValid (Variables|Default|GetEnemyRef)))))

(event Custom|BeginRegen
  (if (Regen|CanPlayerRegen)
    (bind _returnvalue (Utilities|Time|SetTimerbyEvent (delegate Custom|RegenHealth) 1.0 true))
    (Variables|Timers|SetRegenTimerHandle _returnvalue)
    (else
      (Utilities|Time|ClearandInvalidateTimerbyHandle (Variables|Timers|GetRegenTimerHandle)))))

(event Custom|RefOwner
  (bind _returnvalue (Components|GetOwner))
  (if (Actor|ActorHasTag _returnvalue "Player")
    (bind _asbpc_player_character (Utilities|Casting|CastToBPC_PlayerCharacter _returnvalue))
    (Variables|Default|SetPlayerRef _asbpc_player_character)
    (elif (Actor|ActorHasTag _returnvalue "Enemy")
      (bind _asbpc_enemy (Utilities|Casting|CastToBPC_Enemy _returnvalue))
      (Variables|Default|SetEnemyRef _asbpc_enemy))))

(event EventBeginPlay
  (CallFunction|RefOwner))

(fn AddHealth
  (params (Amount :type Float%20%28double-precision%29))
  (Variables|Health|SetCurrentHealth (Math|Float|Clamp(Float) (+ Amount (Variables|Health|GetCurrentHealth)) (Variables|Health|GetMinimumHealth) (Variables|Health|GetMaxHealth))))

(fn RemoveHealth
  (params (Amount :type Float%20%28double-precision%29))
  (bind _output_get (Variables|Health|SetCurrentHealth (Math|Float|Clamp(Float) (- (Variables|Health|GetCurrentHealth) Amount) (Variables|Health|GetMinimumHealth) (Variables|Health|GetMaxHealth))))
  (if (<= _output_get 0.0)
    (return true)
    (else
      (return false))))

(fn CanPlayerRegen
  (if (== (Variables|Regen|GetRegenRate) 0.0)
    (bind _output_get (Variables|Default|SetbRegenEnabled false))
    (return _output_get)
    (elif (< (Variables|Regen|GetRegenRate) 0.0)
      (Variables|HealthState|SetbInjured true)
      (bind _output_get_2 (Variables|Default|SetbRegenEnabled true))
      (return _output_get_2)
      (else
        (bind _output_get_3 (Variables|Default|SetbRegenEnabled true))
        (return _output_get_3)))))

(fn CalculateHealth
  (bind _output_get (Variables|Default|SetHealthPercent (/ (Variables|Health|GetCurrentHealth) (Variables|Health|GetMaxHealth))))
  (return _output_get))

(fn CheckHealth
  (if (< (Health|CalculateHealth) 1.0)
    (return true)
    (else
      (return false))))

(fn SetMaxHealth
  (params (MaxHealth :type Float%20%28double-precision%29))
  (bind _output_get (Variables|Health|SetMaxHealth MaxHealth))
  (if (> (Variables|Health|GetCurrentHealth) _output_get)
    (Variables|Health|SetCurrentHealth _output_get))
  (return))

(fn UpdateRegenRate
  (params (NewRegenRate :type Float%20%28double-precision%29))
  (bind _output_get (Variables|Regen|SetRegenRate NewRegenRate))
  (if (== _output_get 0.0)
    (return)
    (else
      (CallFunction|BeginRegen)
      (return))))