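; Auto-attack component for BPC_PlayerCharacter that periodically fires a sniper projectile at the nearest actor tagged "Enemy".
; After retrying until the owner cast succeeds, it sets a timer from the player's cooldown and fire rate.
; Each cycle computes damage from player stats, picks the closest target and aims, spreading steps across ticks and searching again if none is valid.
; It then spawns BP_Sniper_Projectile from the player's capsule, passes damage, speed and direction, and re-arms the timer.
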(event Custom|GatherTargets
  (Utilities|Time|ClearandInvalidateTimerbyHandle (Variables|Default|GetSnipeTimeHandle))
  (CallFunction|CalculateDamage)
  (bind _outactors (Actor|GetAllActorswithTag "Enemy"))
  (for _array_element _outactors
    (if (< (Transformation|GetDistanceTo (Variables|Default|GetPlayerRef) _array_element) (Variables|Default|GetClosestDistance))
      (Variables|Default|SetClosestDistance (Transformation|GetDistanceTo (Variables|Default|GetPlayerRef) _array_element))
      (Variables|Default|SetClosestEnemy _array_element)))
  (Utilities|FlowControl|DelayUntilNextTick)
  (CallFunction|DetermineVelocity))

(event Custom|PlayerReference
  (bind _asbpc_player_character (Utilities|Casting|CastToBPC_PlayerCharacter (Components|GetOwner))
    (:then
      (Variables|Default|SetPlayerRef _asbpc_player_character)
      (CallFunction|ActivateSniper))
    (:CastFailed
      (Utilities|FlowControl|DelayUntilNextTick)
      (CallFunction|PlayerReference))))

(event Custom|FireSniper
  (Variables|Default|SetClosestDistance 99999999.0)
  (bind _returnvalue (Game|SpawnActorfromClass "/Game/Blueprints/BP_Sniper_Projectile.BP_Sniper_Projectile_C" (Math|Transform|MakeTransform (Transformation|GetWorldLocation (Variables|/Script/Engine.Character|GetCapsuleComponent (Variables|Default|GetPlayerRef))) (Math|Rotator|MakeRotfromX (Variables|Default|GetShotDirection)) "1.000000,1.000000,1.000000") "Undefined" "MultiplyWithRoot" 0 0))
  (Default|DetermineValues _returnvalue (Variables|Default|GetFinalDamage) (Variables|Default|GetProjectileSpeed) (Variables|Default|GetShotDirection) true)
  (CallFunction|ActivateSniper))

(event Custom|DetermineVelocity
  (Utilities|IsValid (Variables|Default|GetClosestEnemy)
    (:Is%20Valid
      (bind _output_get (Variables|Default|SetShotDirection (Math|Vector|GetUnitDirection(Vector) (Transformation|GetActorLocation (Variables|Default|GetPlayerRef)) (Transformation|GetActorLocation (Variables|Default|GetClosestEnemy)))))
      (Variables|Default|SetProjectileVelocity (* _output_get (Variables|Default|GetProjectileSpeed)))
      (Utilities|FlowControl|DelayUntilNextTick)
      (CallFunction|FireSniper))
    (:Is%20Not%20Valid
      (CallFunction|GatherTargets))))

(event Custom|ActivateSniper
  (bind _newfirerate (CallFunction|CalculateTime))
  (bind _returnvalue (Utilities|Time|SetTimerbyEvent (delegate Custom|GatherTargets) _newfirerate))
  (Variables|Default|SetSnipeTimeHandle _returnvalue))

(event EventBeginPlay
  (CallFunction|PlayerReference))

(fn CalculateDamage
  (bind _playerref (Variables|Default|GetPlayerRef))
  (Variables|Default|SetFinalDamage (* (+ (Variables|Default|GetSniperDamage) (Variables|/Game/Blueprints/BPC_PlayerCharacter.BPC_PlayerCharacter_C|GetDamage _playerref)) (Variables|/Game/Blueprints/BPC_PlayerCharacter.BPC_PlayerCharacter_C|GetDamageMultiplier _playerref))))

(fn CalculateTime
  (bind _output_get (Variables|Default|SetCalculatedFireRate (* (Variables|/Game/Blueprints/BPC_PlayerCharacter.BPC_PlayerCharacter_C|GetCooldown (Variables|Default|GetPlayerRef)) (Variables|Default|GetFireRate))))
  (return _output_get))