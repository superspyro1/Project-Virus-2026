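; AC_Health is a health component that tracks an owner's current health.
; AddHealth and RemoveHealth raise or lower CurrentHealth by a given amount, clamping the result between MinimumHealth and MaxHealth.
; Both functions only write the value; the component handles no death or change notification here.
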(fn AddHealth
  (params (Amount :type Float%20%28double-precision%29))
  (Variables|Health|SetCurrentHealth (Math|Float|Clamp(Float) (+ Amount (Variables|Health|GetCurrentHealth)) (Variables|Health|GetMinimumHealth) (Variables|Health|GetMaxHealth))))

(fn RemoveHealth
  (params (Amount :type Float%20%28double-precision%29))
  (Variables|Health|SetCurrentHealth (Math|Float|Clamp(Float) (- (Variables|Health|GetCurrentHealth) Amount) (Variables|Health|GetMinimumHealth) (Variables|Health|GetMaxHealth))))