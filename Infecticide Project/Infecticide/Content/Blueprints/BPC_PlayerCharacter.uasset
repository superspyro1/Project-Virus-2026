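; Player character that holds combat stats, levels up, takes damage and triggers game-over or victory screens.
; Level-ups, including one at BeginPlay, open a card widget offering abilities every five levels or upgrades otherwise.
; Abilities become added components, while upgrades without a required ability modify two stats through enum-driven arithmetic.
; Damage is reduced by Defense or negated with optional spike reflection, health drives the bar, and Tick prints debug stats.
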(event Custom|AchieveVictory
  (bind _controllerref (Variables|Default|GetControllerRef))
  (bind _returnvalue (UserInterface|CreateWidget "/Game/UI/WBP_GameOver.WBP_GameOver_C" _controllerref))
  (UserInterface|Viewport|AddtoViewport _returnvalue 0)
  (Default|SwitchInput _controllerref false _returnvalue))

(event Custom|RefController
  (bind _aspc_player (Utilities|Casting|CastToPC_Player (Game|GetPlayerController 0)))
  (Variables|Default|SetControllerRef _aspc_player))

(event Custom|LevelUp
  (Math|Integer|IncrementInt (Variables|PlayerState|GetCurrentLevel)
    (:%20%20
      (Niagara|SpawnSystematLocation "/Game/Blueprints/FX/Niagara/NS_LevelUp.NS_LevelUp" (Transformation|GetActorLocation))
      (Utilities|FlowControl|Delay 1.0)
      (CallFunction|ChooseUpgrade))))

(event Custom|ChooseUpgrade
  (bind _controllerref (Variables|Default|GetControllerRef))
  (bind _returnvalue (UserInterface|CreateWidget "/Game/UI/WBP_AbilitySelection.WBP_AbilitySelection_C" _controllerref))
  (bind _output_get (Variables|Default|SetAbilitySelection _returnvalue))
  (UserInterface|Viewport|AddtoViewport _output_get 0)
  (Default|SwitchInput _controllerref false _output_get)
  (bind _newability (CallFunction|LevelUpType))
  (if _newability
    (Default|ListCard _output_get "NewEnumerator0")
    (else
      (Default|ListCard _output_get "NewEnumerator1")))
  (EventDispatchers|BindEventtoOnUpgradeSelected (delegate Custom|HIdeAbilitySelection)))

(event Custom|HIdeAbilitySelection
  (params (CardType :type E_CardType%20Enum :default "NewEnumerator0") (AbilityData :type S%20Ability%20Structure) (UpgradeData :type S%20Stat%20Upgrade%20Structure))
  (CallFunction|ApplyChanges CardType AbilityData UpgradeData)
  (Widget|RemovefromParent (Variables|Default|GetAbilitySelection))
  (Default|SwitchInput (Variables|Default|GetControllerRef) true))

(event Custom|ApplyChanges
  (params (CardType :type E_CardType%20Enum :default "NewEnumerator0") (AbilityChanges :type S%20Ability%20Structure) (StatUpgrades :type S%20Stat%20Upgrade%20Structure))
  (switch Utilities|FlowControl|Switch|SwitchonE_CardType CardType
    (:NewEnumerator0
      (CallFunction|AddAbility AbilityChanges))
    (:NewEnumerator1
      (CallFunction|UpgradeStats StatUpgrades))))

(event Custom|DebugPlayerStats
  (bind _ac_health (Variables|Default|GetAC_Health))
  (Development|PrintString (Utilities|String|Append "Damage: " (Utilities|String|ToString(Float) (Variables|Damage|GetDamage))) true true "(R=0.000000,G=0.660000,B=1.000000,A=1.000000)" 0.0)
  (Development|PrintString (Utilities|String|Append "Damage Multiplier: " (Utilities|String|ToString(Float) (Variables|Damage|GetDamageMultiplier))) true true "(R=0.000000,G=0.660000,B=1.000000,A=1.000000)" 0.0)
  (Development|PrintString (Utilities|String|Append "Defense: " (Utilities|String|ToString(Float) (Variables|Defense|GetDefense))) true true "(R=0.000000,G=0.660000,B=1.000000,A=1.000000)" 0.0)
  (Development|PrintString (Utilities|String|Append "Duration:" (Utilities|String|ToString(Float) (Variables|Timing|GetDuration))) true true "(R=0.000000,G=0.660000,B=1.000000,A=1.000000)" 0.0)
  (Development|PrintString (Utilities|String|Append "Cooldown: " (Utilities|String|ToString(Float) (Variables|Timing|GetCooldown))) true true "(R=0.000000,G=0.660000,B=1.000000,A=1.000000)" 0.0)
  (Development|PrintString (Utilities|String|Append "Speed: " (Utilities|String|ToString(Float) (Variables|/Script/Engine.CharacterMovementComponent|GetMaxWalkSpeed (Variables|Character|GetCharacterMovement)))) true true "(R=0.000000,G=0.660000,B=1.000000,A=1.000000)" 0.0)
  (Development|PrintString (Utilities|String|Append "Health: " (Utilities|String|ToString(Float) (Variables|/Game/Blueprints/Components/Attachments/AC_Health.AC_Health_C|GetCurrentHealth _ac_health)) "/" (Utilities|String|ToString(Float) (Variables|/Game/Blueprints/Components/Attachments/AC_Health.AC_Health_C|GetMaxHealth _ac_health))) true true "(R=0.000000,G=0.660000,B=1.000000,A=1.000000)" 0.0)
  (Development|PrintString (Utilities|String|Append "Regen Rate: " (Utilities|String|ToString(Float) (Variables|/Game/Blueprints/Components/Attachments/AC_Health.AC_Health_C|GetRegenRate _ac_health))) true true "(R=0.000000,G=0.660000,B=1.000000,A=1.000000)" 0.0))

(event EventBeginPlay
  (CallFunction|RefController)
  (bind _aswbp_health (Utilities|Casting|CastToWBP_Health (UserInterface|GetUserWidgetObject (Variables|Default|GetHealthBar))))
  (bind _output_get (Variables|Default|SetHealthWidget _aswbp_health))
  (Widget|SetVisibility _output_get "Hidden")
  (CallFunction|LevelUp))

(event EventTick
  (params (DeltaSeconds :type Float%20%28single-precision%29))
  (CallFunction|DebugPlayerStats))

(event EventDealDamage
  (params (Amount :type Float%20%28double-precision%29) (Source :type Actor%20Object%20Reference))
  (bind _self self)
  (bind _healthwidget (Variables|Default|GetHealthWidget))
  (bind _returnvalue (Actor|GetComponentbyClass _self "/Game/Blueprints/Components/Abilities/SpikeBody/AC_SpikeBody.AC_SpikeBody_C"))
  (if (Variables|Default|GetbNegateDamage)
    (Utilities|IsValid _returnvalue
      (:Is%20Valid
        (Class|BPICombat|DealDamage(Message) Source (Variables|/Game/Blueprints/Components/Abilities/SpikeBody/AC_SpikeBody.AC_SpikeBody_C|GetFinalDamage _returnvalue) self)
        (Development|PrintString "Hello")))
    (else
      (CallFunction|DamageIndicator)
      (bind _finaldamage (CallFunction|CalculateDamage Amount))
      (bind _dead_ (Default|RemoveHealth (Variables|Default|GetAC_Health) _finaldamage))
      (if _dead_
        (bind _returnvalue_2 (UserInterface|CreateWidget "/Game/UI/WBP_GameOver.WBP_GameOver_C" (Game|GetPlayerController 0)))
        (UserInterface|Viewport|AddtoViewport _returnvalue_2 0)
        (Game|SetGamePaused true)
        (else
          (if (Default|CheckHealth (Variables|Default|GetAC_Health))
            (Widget|SetVisibility _healthwidget "Visible")
            (else
              (Widget|SetVisibility _healthwidget "Hidden")))
          (CallFunction|UpdateHealthWidget))))))

(event EventHealDamage
  (params (Amount :type Float%20%28double-precision%29) (Source :type Actor%20Object%20Reference))
  (bind _healthwidget (Variables|Default|GetHealthWidget))
  (Default|AddHealth (Variables|Default|GetAC_Health) Amount)
  (if (Default|CheckHealth (Variables|Default|GetAC_Health))
    (Widget|SetVisibility _healthwidget "Visible")
    (else
      (Widget|SetVisibility _healthwidget "Hidden")))
  (CallFunction|UpdateHealthWidget))

(fn ConstructionScript)

(fn CalculateDamage
  (params (IncomingDamage :type Float%20%28double-precision%29))
  (return (Math|Float|Clamp(Float) (- IncomingDamage (Variables|Defense|GetDefense)) 0.0 1e+19)))

(fn UpdateHealthWidget
  (Default|UpdateHealthBar (Variables|Default|GetHealthWidget) (Default|CalculateHealth (Variables|Default|GetAC_Health))))

(fn DamageIndicator
  (Niagara|SpawnSystematLocation "/Game/Blueprints/FX/Niagara/NS_HitDetection.NS_HitDetection" (Transformation|GetActorLocation) (Math|Random|RandomRotator false)))

(fn AddAbility
  (params (Ability :type S%20Ability%20Structure))
  (Game|AddComponentbyClass (Utilities|Struct|BreakS_Ability Ability))
  (return))

(fn UpgradeStats
  (params (NewUpgrades :type S%20Stat%20Upgrade%20Structure))
  (bind (_cardname _cardinfo _cardimage _primary _primaryvalue _primaryapplication _secondary _secondaryvalue _secondaryapplication _requiredability) (Utilities|Struct|BreakS_StatUpgrade NewUpgrades))
  (if (not (Utilities|IsValidClass _requiredability))
    (bind _stattype (CallFunction|DetermineStattoChange _primary))
    (bind _result (CallFunction|ApplyModifier _primaryapplication _stattype _primaryvalue))
    (CallFunction|UpdateStats _primary _result)
    (bind _stattype_2 (CallFunction|DetermineStattoChange _secondary))
    (bind _result_2 (CallFunction|ApplyModifier _secondaryapplication _stattype_2 _secondaryvalue))
    (CallFunction|UpdateStats _secondary _result_2)))

(fn Add
  (params (A :type Float%20%28double-precision%29) (B :type Float%20%28double-precision%29))
  (return (+ A B)))

(fn Subtract
  (params (A :type Float%20%28double-precision%29) (B :type Float%20%28double-precision%29))
  (return (- A B)))

(fn Divide
  (params (A :type Float%20%28double-precision%29) (B :type Float%20%28double-precision%29))
  (return (/ A B)))

(fn Multiply
  (params (A :type Float%20%28double-precision%29) (B :type Float%20%28double-precision%29))
  (return (* A B)))

(fn ApplyModifier
  (params (ApplicationMethod :type E_ApplicationType%20Enum :default "NewEnumerator0") (Stat :type Float%20%28double-precision%29) (Change :type Float%20%28double-precision%29))
  (switch Utilities|FlowControl|Switch|SwitchonE_ApplicationType ApplicationMethod
    (:NewEnumerator0
      (return (Operator|Add Stat Change)))
    (:NewEnumerator1
      (return (Operator|Subtract Stat Change)))
    (:NewEnumerator2
      (return (Operator|Multiply Stat Change)))
    (:NewEnumerator3
      (return (Operator|Divide Stat Change)))))

(fn DetermineStattoChange
  (params (StatChange :type E_StatType%20Enum :default "NewEnumerator0"))
  (bind _ac_health (Variables|Default|GetAC_Health))
  (switch Utilities|FlowControl|Switch|SwitchonE_StatType StatChange
    (:NewEnumerator0
      (return 0.0))
    (:NewEnumerator1
      (return (Variables|Damage|GetDamage)))
    (:NewEnumerator2
      (return (Variables|/Game/Blueprints/Components/Attachments/AC_Health.AC_Health_C|GetMaxHealth _ac_health)))
    (:NewEnumerator3
      (return (Class|MovementComponent|GetMaxSpeed (Variables|Character|GetCharacterMovement))))
    (:NewEnumerator4
      (return (Variables|Timing|GetCooldown)))
    (:NewEnumerator6
      (return (Variables|Timing|GetDuration)))
    (:NewEnumerator5
      (return (Variables|Defense|GetDefense)))
    (:NewEnumerator7
      (return (Variables|/Game/Blueprints/Components/Attachments/AC_Health.AC_Health_C|GetRegenRate _ac_health)))
    (:NewEnumerator8
      (return (Variables|Damage|GetDamageMultiplier)))))

(fn UpdateStats
  (params (StatType :type E_StatType%20Enum :default "NewEnumerator0") (NewValue :type Float%20%28double-precision%29))
  (bind _ac_health (Variables|Default|GetAC_Health))
  (bind _ac_health_2 (Variables|Default|GetAC_Health))
  (switch Utilities|FlowControl|Switch|SwitchonE_StatType StatType
    (:NewEnumerator0
      _)
    (:NewEnumerator1
      (Variables|Damage|SetDamage NewValue))
    (:NewEnumerator2
      (bind _output_get (Variables|/Game/Blueprints/Components/Attachments/AC_Health.AC_Health_C|SetMaxHealth _ac_health_2 NewValue))
      (Default|SetMaxHealth _ac_health_2 _output_get))
    (:NewEnumerator3
      (Variables|/Script/Engine.CharacterMovementComponent|SetMaxWalkSpeed (Variables|Character|GetCharacterMovement) NewValue))
    (:NewEnumerator4
      (Variables|Timing|SetCooldown NewValue))
    (:NewEnumerator6
      (Variables|Timing|SetDuration NewValue))
    (:NewEnumerator5
      (Variables|Defense|SetDefense NewValue))
    (:NewEnumerator7
      (bind _output_get_2 (Variables|/Game/Blueprints/Components/Attachments/AC_Health.AC_Health_C|SetRegenRate _ac_health NewValue))
      (Default|UpdateRegenRate _ac_health _output_get_2))
    (:NewEnumerator8
      (Variables|Damage|SetDamageMultiplier NewValue)))
  (return))

(fn LevelUpType
  (if (== (Variables|PlayerState|GetCurrentLevel) (Variables|PlayerState|GetNewAbilityLevel))
    (Variables|PlayerState|SetNewAbilityLevel (+ (Variables|PlayerState|GetCurrentLevel) 5))
    (return true)
    (else
      (return false))))