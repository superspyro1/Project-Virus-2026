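; Player controller that adds the gameplay Enhanced Input mapping context and possesses the player character placed in the world.
; On BeginPlay it looks up BPC_PlayerCharacter, retrying each tick until one exists before possessing it.
; The move action drives the character along its Body component's right and forward vectors.
; SwitchInput toggles between unpaused game-only input and paused UI-only input with a visible cursor focused on a given widget.
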(event Custom|AddMappingContext
  (Input|AddMappingContext (PlayerController|LocalPlayerSubsystems|GetEnhancedInputLocalPlayerSubsystem (Game|GetPlayerController 0)) "/Game/Blueprints/Controller/IMC_Gameplay.IMC_Gameplay" 0 "(bIgnoreAllPressedKeysUntilRelease=True,bForceImmediately=False,bNotifyUserSettings=False)"))

(event Custom|PossessPlayer
  (bind _returnvalue (Actor|GetActorOfClass "/Game/Blueprints/BPC_PlayerCharacter.BPC_PlayerCharacter_C"))
  (Utilities|IsValid _returnvalue
    (:Is%20Valid
      (bind _output_get (Variables|Default|SetPlayerCharacter _returnvalue))
      (Pawn|Possess _output_get))
    (:Is%20Not%20Valid
      (Utilities|FlowControl|DelayUntilNextTick)
      (CallFunction|PossessPlayer))))

(event EventBeginPlay
  (CallFunction|AddMappingContext)
  (CallFunction|PossessPlayer))

(event Input|EnhancedActionEvents|EnhancedInputActionIA_Move
  (params (ActionValue :type Vector%202D%20Structure) (ElapsedSeconds :type Float%20%28double-precision%29) (TriggeredSeconds :type Float%20%28double-precision%29) (InputAction :type Input%20Action%20Object%20Reference :default "/Game/Blueprints/Controller/Inputs/IA_Move.IA_Move"))
  (bind _playercharacter (Variables|Default|GetPlayerCharacter))
  (Pawn|Input|AddMovementInput _playercharacter (Math|Vector|GetRightVector (Variables|/Game/Blueprints/BPC_PlayerCharacter.BPC_PlayerCharacter_C|GetBody _playercharacter)) (.x ActionValue) false)
  (Pawn|Input|AddMovementInput _playercharacter (Math|Vector|GetForwardVector (Variables|/Game/Blueprints/BPC_PlayerCharacter.BPC_PlayerCharacter_C|GetBody _playercharacter)) (.y ActionValue) false))

(fn ConstructionScript)

(fn SwitchInput
  (params (Gameplay :type Boolean) (Widget :type Widget%20Object%20Reference))
  (bind _returnvalue (Game|GetPlayerController 0))
  (if Gameplay
    (Input|SetInputModeGameOnly _returnvalue false)
    (Variables|/Script/Engine.PlayerController|SetbShowMouseCursor _returnvalue false)
    (Game|SetGamePaused false)
    (else
      (Input|SetInputModeUIOnly _returnvalue Widget "DoNotLock" false)
      (Variables|/Script/Engine.PlayerController|SetbShowMouseCursor _returnvalue true)
      (Game|SetGamePaused true))))