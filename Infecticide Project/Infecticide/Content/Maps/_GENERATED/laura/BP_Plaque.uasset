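; Plaque actor that continuously morphs between random, non-uniform scales.
; A timer picks the next target scale and, after a short delay, plays a timeline that lerps the actor from its previous scale, then restarts the cycle on finish.
; On overlap, its collision switches to query-only for another actor of the same class and to query-and-physics for anything else.
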(event OnComponentBeginOverlap(Collision)
  (params (OverlappedComponent :type Primitive%20Component%20Object%20Reference) (OtherActor :type Actor%20Object%20Reference) (OtherComp :type Primitive%20Component%20Object%20Reference) (OtherBodyIndex :type Integer) (bFromSweep :type Boolean) (SweepResult :type Hit%20Result%20Structure%20%28by%20ref%29))
  (bind _collision (Variables|Default|GetCollision))
  (if (== (Utilities|GetClass OtherActor) (Utilities|GetClass self))
    (Collision|SetCollisionEnabled _collision "QueryOnly")
    (else
      (Collision|SetCollisionEnabled _collision "QueryAndPhysics"))))

(event Custom|ScaleTimer
  (CallFunction|CalculateScale)
  (bind _returnvalue (Utilities|Time|SetTimerbyEvent (delegate Custom|ChangeScale) 1.0))
  (Variables|Default|SetScaleTimerHandle _returnvalue))

(event Custom|ChangeScale
  (Utilities|Time|ClearandInvalidateTimerbyHandle (Variables|Default|GetScaleTimerHandle))
  (bind _newtrack_0 (Timeline|ScaleTime PlayFromStart)
    (:Update
      (CallFunction|AnimateScale _newtrack_0))
    (:Finished
      (CallFunction|ScaleTimer))))

(event EventBeginPlay
  (CallFunction|ScaleTimer))

(fn ConstructionScript)

(fn AnimateScale
  (params (Time :type Float%20%28double-precision%29))
  (Transformation|SetActorScale3D (Math|Vector|Lerp(Vector) (Variables|Default|GetOldScale) (Variables|Default|GetNewScale) Time)))

(fn CalculateScale
  (Variables|Default|SetOldScale (Variables|Default|GetNewScale))
  (Variables|Default|SetNewScale (Math|Vector|MakeVector (Math|Random|RandomFloatinRange 2.5 3.0) (Math|Random|RandomFloatinRange 2.5 3.0) (Math|Random|RandomFloatinRange 2.0 3.0)))
  (return))